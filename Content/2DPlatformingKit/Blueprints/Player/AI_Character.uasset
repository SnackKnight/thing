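; AI-controlled 2D platformer character that moves toward any Player_Character its PawnSensing spots, alongside a full set of player-style systems.
; Number keys equip owned weapons, swapping projectile and melee classes and highlighting HUD icons.
; Timed power-ups use retriggerable delays to alter damage, vulnerability or jumping, or enable Bad Touch overlap damage, also granted by landing impacts.
; XP drives table-based level-ups that raise health and redraw widget icons.
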(event OnSeePawn(PawnSensing)
  (params (Pawn :type Pawn%20Object%20Reference))
  (bind _asplayer_character (Utilities|Casting|CastToPlayer_Character Pawn))
  (AI|AIMoveTo self "0, 0, 0" _asplayer_character 1e+01 false))

(event OnComponentBeginOverlap(CapsuleComponent)
  (params (OverlappedComponent :type Primitive%20Component%20Object%20Reference) (OtherActor :type Actor%20Object%20Reference) (OtherComp :type Primitive%20Component%20Object%20Reference) (OtherBodyIndex :type Integer) (bFromSweep :type Boolean) (SweepResult :type Hit%20Result%20Structure%20%28by%20ref%29))
  ;[1 1 1] If Bad Touch is active then damage enemies that overlap you!
  (if (Variables|PowerUps|GetIsBadTouchActive)
    (if (Actor|ActorHasTag OtherActor (Variables|PowerUps|GetDestroyableTag))
      ;;[0.1595 0.2271 1] Blueprint Interface Call
      (Class|InteractionHandler|ActorDamagedbyObject(Message) OtherActor (Variables|PowerUps|GetBadTouchDamage) "0, 0, 0")
      ;;[0.1595 0.2271 1] Spawn Hit FX
      (Effects|SpawnEmitteratLocation (Variables|PowerUps|GetBadTouchHitFX) (Transformation|GetWorldLocation (Variables|Collision|GetCapsuleComponent))))))

(event EventGrantPowerUp
  (params (PowerUp :type power_up_list%20Enum :default "NewEnumerator0") (Duration :type Float%20%28single-precision%29))
  ;[1 1 1] PowerUpHandler
  (Development|PrintString (Utilities|String|Append (Utilities|String|EnumtoString PowerUp) " for " (Utilities|String|ToString(Float) Duration) " seconds!"))
  (switch Utilities|FlowControl|Switch|Switchonpower_up_list PowerUp
    (:NewEnumerator0
      ;;[0 0.03607 1] Multiply player damage for the duration
      (Variables|DoNotModify!|SetCurrentDamageMultiplier (Variables|PowerUps|GetSuperDamageMultiplier))
      (Utilities|FlowControl|RetriggerableDelay Duration)
      (Variables|DoNotModify!|SetCurrentDamageMultiplier (Variables|Editable|GetDefaultDamageMultiplier)))
    (:NewEnumerator1
      ;;[0 0.03607 1] Make the player Invulnerable for the duration
      (Variables|PowerUps|SetIsPlayerVulnerable false)
      (Utilities|FlowControl|RetriggerableDelay Duration)
      (Variables|PowerUps|SetIsPlayerVulnerable true))
    (:NewEnumerator2
      ;;[0 0.03607 1] Make the player jump higher for the duration
      (Variables|/Script/Engine.CharacterMovementComponent|SetJumpZVelocity (Variables|Character|GetCharacterMovement) (Variables|PowerUps|GetSuperJumpVelocity))
      (Utilities|FlowControl|RetriggerableDelay Duration)
      (Variables|/Script/Engine.CharacterMovementComponent|SetJumpZVelocity (Variables|Character|GetCharacterMovement) (Variables|DoNotModify!|GetDefaultJumpVelocity)))
    (:NewEnumerator3
      ;;[0 0.03607 1] Give the player multi jump for the duration
      (Variables|DoNotModify!|SetmaxJumps (Variables|PowerUps|GetMultiJumpAmount))
      (Utilities|FlowControl|RetriggerableDelay Duration)
      (Variables|DoNotModify!|SetmaxJumps (Variables|Editable|GetDefaultJumpAmount)))
    (:NewEnumerator5
      ;;[0 0.03607 1] Make the player invulnerable to enemy damage and allow him to kill enemies just by touching them.
      (Variables|PowerUps|SetIsBadTouchActive true)
      (Utilities|FlowControl|RetriggerableDelay Duration)
      (Variables|PowerUps|SetIsBadTouchActive false)))
  ;;[1 1 1] Debug information. Can be deleted
  (Development|PrintString (Utilities|String|Append (Utilities|String|EnumtoString PowerUp) " expired!")))

(event Input|KeyboardEvents|3
  (params (Key :type Key%20Structure :default "None"))
  (bind _weaponidllist (Variables|Weapons|GetWeaponIDlList))
  ;[1 1 1] Use number keys to swap between the weapons. Each weapon will spawn it's own unique projectile and melee damage zone.
  (:Released
    (if (Utilities|Array|IsValidIndex _weaponidllist 2)
      (bind _weaponavailable (CallFunction|EquipWeapon (Utilities|Array|Get(acopy) _weaponidllist 2)))
      (if _weaponavailable
        (CallFunction|EquipWeaponIcons 2)
        (Variables|Editable|SetrangedProjectileClass (Variables|Weapons|GetPurpleSwordRangedProjectile))
        (Variables|Editable|SetmeleeDamageZoneClass (Variables|Weapons|GetPurpleSwordMeleeZone))))))

(event Input|KeyboardEvents|1
  (params (Key :type Key%20Structure :default "None"))
  ;[1 1 1] Use number keys to swap between the weapons. Each weapon will spawn it's own unique projectile and melee damage zone.
  (:Released
    (bind _weaponavailable (CallFunction|EquipWeapon (Utilities|Array|Get(acopy) (Variables|Weapons|GetWeaponIDlList))))
    (if _weaponavailable
      (CallFunction|EquipWeaponIcons)
      (Variables|Editable|SetrangedProjectileClass (Variables|Weapons|GetDefaultSwordRangedProjectile))
      (Variables|Editable|SetmeleeDamageZoneClass (Variables|Weapons|GetDefaultSwordMeleeZone)))))

(event Input|KeyboardEvents|2
  (params (Key :type Key%20Structure :default "None"))
  (bind _weaponidllist (Variables|Weapons|GetWeaponIDlList))
  ;[1 1 1] Use number keys to swap between the weapons. Each weapon will spawn it's own unique projectile and melee damage zone.
  (:Released
    (if (Utilities|Array|IsValidIndex _weaponidllist 1)
      (bind _weaponavailable (CallFunction|EquipWeapon (Utilities|Array|Get(acopy) _weaponidllist 1)))
      (if _weaponavailable
        (CallFunction|EquipWeaponIcons 1)
        (Variables|Editable|SetrangedProjectileClass (Variables|Weapons|GetOrangeSwordRangedProjectile))
        (Variables|Editable|SetmeleeDamageZoneClass (Variables|Weapons|GetOrangeSwordMeleeZone))))))

(fn ConstructionScript
  ;[1 1 1] Set the maximum number of jumps and initial movespeed.
  (Variables|DoNotModify!|SetcurrentJumps (Variables|DoNotModify!|GetmaxJumps))
  (Variables|DoNotModify!|SetinitialMoveSpeed (Variables|/Script/Engine.CharacterMovementComponent|GetMaxWalkSpeed (Variables|Character|GetCharacterMovement)))
  (Variables|Editable|SetoffsethealthX (Variables|Editable|GetoffsethealthBackgroundX)))

(fn DrawHealthBackground
  (bind _healthbackgroundarray (Variables|DoNotModify!|GethealthBackgroundArray))
  ;[1 1 1] Drawn health background graphics
  (Widget|RemovefromParent _healthbackgroundarray)
  (Utilities|Array|Clear _healthbackgroundarray)
  (for _index (range 1 (Variables|Editable|GetplayerHealthMax))
    (bind _returnvalue (UserInterface|CreateWidget "/Game/2DPlatformingKit/Widgets/healthDepleted.healthDepleted_C" (Game|GetPlayerController 0)))
    (Utilities|Array|Add (Variables|DoNotModify!|GethealthBackgroundArray) _returnvalue)
    (UserInterface|Viewport|AddtoViewport _returnvalue 0)
    (Class|UserWidget|SetPositioninViewport _returnvalue (Math|Vector2D|MakeVector2D (Variables|Editable|GetoffsethealthBackgroundX) 0.0) false)
    (Variables|Editable|SetoffsethealthBackgroundX (+ (Variables|Editable|GetoffsethealthBackgroundX) 33.0)))
  (Variables|Editable|SetoffsethealthBackgroundX 0.0))

(fn DrawHealth
  (bind _healthiconarray (Variables|DoNotModify!|GethealthIconArray))
  ;[1 1 1] Draw Health Graphics
  (Widget|RemovefromParent _healthiconarray)
  (Utilities|Array|Clear _healthiconarray)
  (if (> (Variables|DoNotModify!|GetplayerHealthCurrent) (Variables|Editable|GetplayerHealthMax))
    (Variables|DoNotModify!|SetplayerHealthCurrent (Variables|Editable|GetplayerHealthMax)))
  (for _index (range 1 (Variables|DoNotModify!|GetplayerHealthCurrent))
    (bind _returnvalue (UserInterface|CreateWidget "/Game/2DPlatformingKit/Widgets/healthFull.healthFull_C" (Game|GetPlayerController 0)))
    (Utilities|Array|Add (Variables|DoNotModify!|GethealthIconArray) _returnvalue)
    ;;[0.1595 0.2271 1] Draw and offset Health Graphics
    (UserInterface|Viewport|AddtoViewport _returnvalue 1)
    (Class|UserWidget|SetPositioninViewport _returnvalue (Math|Vector2D|MakeVector2D (Variables|Editable|GetoffsethealthX) 0.0) false)
    (Variables|Editable|SetoffsethealthX (+ (Variables|Editable|GetoffsethealthX) 33.0)))
  (Variables|Editable|SetoffsethealthX 0.0))

(fn PlayerDeath
  ;[1 1 1] Destroy the player sprite and enable the game over text
  (Components|DestroyComponent (Variables|Default|GetSprite))
  (Variables|DoNotModify!|SetisPlayerDead true)
  (Collision|SetCollisionEnabled (Variables|Collision|GetCapsuleComponent) "NoCollision")
  (Pawn|Components|CharacterMovement|DisableMovement (Variables|Character|GetCharacterMovement))
  (Components|Activation|SetActive true false)
  (Input|DisableInput 0)
  (Default|PlayerDied (Variables|DoNotModify!|GetHUD) (Variables|Editable|GettouchButtonsEnabled?)))

(fn EquipWeapon
  (params (WeaponID :type Byte))
  (bind _weaponlist (Variables|Weapons|GetWeaponList))
  ;[1 1 1] Unequip all weapons
  (bind (_array_element _array_index) (Utilities|Array|ForEachLoopwithBreak _weaponlist)
    (:LoopBody
      (Utilities|Array|SetArrayElem _weaponlist _array_index (Utilities|Struct|MakeWeaponStructure (.WeaponID (Utilities|Struct|BreakWeaponStructure _array_element)) (.WeaponName (Utilities|Struct|BreakWeaponStructure _array_element)) (.WeaponIcon (Utilities|Struct|BreakWeaponStructure _array_element)) (.PlayerHasWeapon (Utilities|Struct|BreakWeaponStructure _array_element)))))
    (:Completed
      ;[1 1 1] Search for the weapon with the corresponding ID and see if the player has the weapon
      (bind (_array_element_2 _array_index_2) (Utilities|Array|ForEachLoopwithBreak (Variables|Weapons|GetWeaponList))
        (:LoopBody
          (if (== (.WeaponID (Utilities|Struct|BreakWeaponStructure _array_element_2)) WeaponID)
            (LocalVariables|SetfoundweaponID true)
            (if (.PlayerHasWeapon (Utilities|Struct|BreakWeaponStructure _array_element_2))
              ;[1 1 1] If player has the weapon then equip it else display error messages!
              (Utilities|Array|SetArrayElem (Variables|Weapons|GetWeaponList) _array_index_2 (Utilities|Struct|MakeWeaponStructure (.WeaponID (Utilities|Struct|BreakWeaponStructure _array_element_2)) (.WeaponName (Utilities|Struct|BreakWeaponStructure _array_element_2)) 0 (.PlayerHasWeapon (Utilities|Struct|BreakWeaponStructure _array_element_2)) true))
              (Development|PrintString (Utilities|String|Append "Player equipped : " (Utilities|String|ToString(Text) (.WeaponName (Utilities|Struct|BreakWeaponStructure _array_element_2)))))
              (Variables|Weapons|SetEquippedWeaponID (Math|Conversions|ToInteger(Byte) (.WeaponID (Utilities|Struct|BreakWeaponStructure _array_element_2))))
              (else
                (Development|PrintString "Weapon Not Available")
                (LocalVariables|SetWeaponAvailable? false)))
            (return (LocalVariables|GetWeaponAvailable?))))
        (:Completed
          (if (LocalVariables|GetfoundweaponID)
            _
            (else
              (Development|PrintString "Invalid Weapon ID!")
              (LocalVariables|SetWeaponAvailable? false)))
          (return (LocalVariables|GetWeaponAvailable?)))))))

(fn PickUpWeapon
  (params (WeaponID :type Byte))
  ;[1 1 1] Find weapon with matching ID
  (bind (_array_element _array_index) (Utilities|Array|ForEachLoopwithBreak (Variables|Weapons|GetWeaponList))
    (:LoopBody
      (if (== WeaponID (.WeaponID (Utilities|Struct|BreakWeaponStructure _array_element)))
        ;[1 1 1] If weapon is valid then equip it and add the icon to the HUD
        (Utilities|Array|SetArrayElem (Variables|Weapons|GetWeaponList) _array_index (Utilities|Struct|MakeWeaponStructure (.WeaponID (Utilities|Struct|BreakWeaponStructure _array_element)) (.WeaponName (Utilities|Struct|BreakWeaponStructure _array_element)) (.WeaponIcon (Utilities|Struct|BreakWeaponStructure _array_element)) true (.PlayerHasWeaponEquipped (Utilities|Struct|BreakWeaponStructure _array_element))))
        (Development|PrintString (Utilities|String|Append "Player picked-up : " (Utilities|String|ToString(Text) (.WeaponName (Utilities|Struct|BreakWeaponStructure _array_element)))))
        (CallFunction|AddWeaponIcons (.WeaponIcon (Utilities|Struct|BreakWeaponStructure (Utilities|Struct|MakeWeaponStructure (.WeaponID (Utilities|Struct|BreakWeaponStructure _array_element)) (.WeaponName (Utilities|Struct|BreakWeaponStructure _array_element)) (.WeaponIcon (Utilities|Struct|BreakWeaponStructure _array_element)) true (.PlayerHasWeaponEquipped (Utilities|Struct|BreakWeaponStructure _array_element))))) (.WeaponID (Utilities|Struct|BreakWeaponStructure (Utilities|Struct|MakeWeaponStructure (.WeaponID (Utilities|Struct|BreakWeaponStructure _array_element)) (.WeaponName (Utilities|Struct|BreakWeaponStructure _array_element)) (.WeaponIcon (Utilities|Struct|BreakWeaponStructure _array_element)) true (.PlayerHasWeaponEquipped (Utilities|Struct|BreakWeaponStructure _array_element))))))
        (Utilities|Array|AddUnique (Variables|Weapons|GetWeaponIDlList) (.WeaponID (Utilities|Struct|BreakWeaponStructure (Utilities|Struct|MakeWeaponStructure (.WeaponID (Utilities|Struct|BreakWeaponStructure _array_element)) (.WeaponName (Utilities|Struct|BreakWeaponStructure _array_element)) (.WeaponIcon (Utilities|Struct|BreakWeaponStructure _array_element)) true (.PlayerHasWeaponEquipped (Utilities|Struct|BreakWeaponStructure _array_element))))))
        (return)))
    (:Completed
      (Development|PrintString "Weapon not found!")
      (return))))

(fn AddWeaponIcons
  (params (WeaponIcon :type Texture%202D%20Object%20Reference) (WeaponID :type Byte))
  ;[1 1 1] Draw Weapon graphics
  (bind _returnvalue (UserInterface|CreateWidget "/Game/2DPlatformingKit/Widgets/WeaponWidget.WeaponWidget_C" (Game|GetPlayerController 0)))
  (Variables|/Game/2DPlatformingKit/Widgets/WeaponWidget.WeaponWidget_C|SetweaponImage _returnvalue WeaponIcon)
  (Variables|/Game/2DPlatformingKit/Widgets/WeaponWidget.WeaponWidget_C|SetWeaponID _returnvalue WeaponID)
  (Utilities|Array|Add (Variables|Weapons|GetWeaponIconArray) _returnvalue)
  ;;[0.1595 0.2271 1] Draw and offset Health Graphics
  (UserInterface|Viewport|AddtoViewport _returnvalue 3)
  (Class|UserWidget|SetPositioninViewport _returnvalue (Math|Vector2D|MakeVector2D (Variables|Weapons|GetOffsetWeaponX) 175.0) false)
  (Variables|Weapons|SetOffsetWeaponX (+ 55.0 (Variables|Weapons|GetOffsetWeaponX)))
  (return))

(fn EquipWeaponIcons
  (params (WeaponIconArrayElement :type Integer))
  (bind _weaponiconarray (Variables|Weapons|GetWeaponIconArray))
  (bind _output (Utilities|Array|Get(acopy) _weaponiconarray WeaponIconArrayElement))
  ;[1 1 1] Reset all icons then increase the alpha of the selected weapon
  (for _array_element (Variables|Weapons|GetWeaponIconArray)
    (Variables|/Game/2DPlatformingKit/Widgets/WeaponWidget.WeaponWidget_C|SetweaponImageBrush _array_element (Variables|/Game/2DPlatformingKit/Widgets/WeaponWidget.WeaponWidget_C|GetweaponImageBrushDefault _array_element)))
  ;;[1 1 1] checks if array id is within range
  (if (< WeaponIconArrayElement (Utilities|Array|Length (Variables|Weapons|GetWeaponIconArray)))
    (Variables|/Game/2DPlatformingKit/Widgets/WeaponWidget.WeaponWidget_C|SetweaponImageBrush _output (Utilities|Struct|MakeLinearColor (.R (Utilities|Struct|BreakLinearColor (Variables|/Game/2DPlatformingKit/Widgets/WeaponWidget.WeaponWidget_C|GetweaponImageBrush _output))) (.G (Utilities|Struct|BreakLinearColor (Variables|/Game/2DPlatformingKit/Widgets/WeaponWidget.WeaponWidget_C|GetweaponImageBrush _output))) (.B (Utilities|Struct|BreakLinearColor (Variables|/Game/2DPlatformingKit/Widgets/WeaponWidget.WeaponWidget_C|GetweaponImageBrush _output))) 1.0))))

(fn CanJumpInternal
  (bind _returnvalue (|CallParentFunction))
  (return (or _returnvalue (Class|NavMovementComponent|IsFlying (Variables|Character|GetCharacterMovement)))))

(fn LandingImpact
  (params (InvulnerabilityDuration :type Float%20%28single-precision%29))
  (bind _returnvalue (Transformation|GetActorLocation))
  (Effects|SpawnEmitteratLocation "/Game/2DPlatformingKit/FX/Impact.Impact" _returnvalue)
  (Camera|PlayWorldCameraShake "/Game/2DPlatformingKit/Blueprints/Player/PlayerShake.PlayerShake_C" _returnvalue 0.0 1e+03)
  (CallFunction|GrantPowerUp "NewEnumerator5" InvulnerabilityDuration))

(fn EarnXP
  (params (XP :type Integer))
  (bind _output_get (Variables|Editable|SetcurrentXP (+ XP (Variables|Editable|GetcurrentXP))))
  ;[1 1 1] Check to see if we require multiple level ups
  (if (>= _output_get (Utilities|Array|Get(acopy) (Variables|Editable|GetExperienceTable) (- (Variables|Editable|GetplayerLevel) 0))) :!label _label
    (Variables|Editable|SetplayerLevel (+ (Variables|Editable|GetplayerLevel) 1))
    (CallFunction|LevelUpStats (Variables|Editable|GetHealthPerLevel))
    (Class|UICommunication|LevelUp(Message) (Variables|DoNotModify!|GetHUD) (Variables|Editable|GetplayerLevel))
    (goto _label)))

(fn LevelUpStats
  (params (Health :type Integer))
  (bind _output_get (Variables|Editable|SetplayerHealthMax (+ Health (Variables|Editable|GetplayerHealthMax))))
  (Variables|DoNotModify!|SetplayerHealthCurrent _output_get)
  (Game|SpawnActorfromClass "/Game/2DPlatformingKit/Blueprints/Player/LevelUp.LevelUp_C" (Transformation|GetWorldTransform (Variables|Default|GetLevelupPos)) "Undefined" 0 0)
  (Audio|PlaySound2D "/Game/2DPlatformingKit/SFX/LevelUp.LevelUp" 1.0 1.0 0.0 0 0)
  (CallFunction|DrawHealthBackground)
  (CallFunction|DrawHealth))